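; SplineRiver is an environment Blueprint for the UndeadVillage set that builds a river, as its name indicates, along a spline.
; The construction script adds one spline mesh component per segment between consecutive spline points, attached to the scene root.
; Each segment takes its start and end positions and tangents from the spline's local point data, so it bends along the curve.
; The event graph has no runtime logic.
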(fn `UserConstructionScript`
  (bind _spline (`self.Spline`))
  (for _index (range (+ (- (`SplineComponent.GetNumberOfSplinePoints` _spline) 2) 1))
    (bind _returnvalue (`AddComponent|NODE_AddSplineMeshComponent-0`))
    (`SceneComponent.K2_AttachTo` _returnvalue (`self.DefaultSceneRoot`) "None" "KeepRelativeOffset" false)
    (bind (_locallocation _localtangent) (`SplineComponent.GetLocalLocationAndTangentAtSplinePoint` _spline _index))
    (bind (_locallocation_2 _localtangent_2) (`SplineComponent.GetLocalLocationAndTangentAtSplinePoint` _spline (+ _index 1)))
    (`SplineMeshComponent.SetStartAndEnd` _returnvalue _locallocation _localtangent _locallocation_2 _localtangent_2 true)))