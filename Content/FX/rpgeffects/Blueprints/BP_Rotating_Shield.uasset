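; Rotating shield effect Blueprint that circles a ring of particle effects around an arrow component.
; The construction script spawns one particle component per shield level, spaced evenly by yaw, with configurable template and scale.
; Each is pushed out along its local X by the shield radius and attached to the arrow.
; Tick spins the arrow in world yaw by a fixed step per frame, not scaled by delta time.
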(event `self.ReceiveTick`
  (params (DeltaSeconds :type "Float (single-precision)"))
  ;[1 1 1] RotateSystem
  (`SceneComponent.K2_AddWorldRotation` (`self.Arrow`) (`KismetMathLibrary.MakeRotator` 0.0 0.0 (`self.Shield_RotateSpeed`)) false false))

(fn `UserConstructionScript`
  (locals (CurrentParticleEffect :type "ParticleSystemComponent Object Reference") (DegreesInACircle :type "Float (double-precision)" :default 360.0) (RotationAngle :type "Float (double-precision)"))
  ;[1 1 1] Setup Initial Particle Effects
  (set `local.RotationAngle` (/ (`local.DegreesInACircle`) (`KismetMathLibrary.Conv_IntToDouble` (`self.Shield_Level`))))
  (for _index (range 1 (+ (`self.Shield_Level`) 1))
    (bind _returnvalue (`AddComponent|NODE_AddParticleSystemComponent-0` :`RelativeTransform` (`KismetMathLibrary.MakeTransform` (0.0 0.0 0.0) (`KismetMathLibrary.MakeRotator` 0.0 0.0 (* _index (`local.RotationAngle`))))))
    (bind _output_get (set `local.CurrentParticleEffect` _returnvalue))
    (`ParticleSystemComponent.SetTemplate` _output_get (`self.ParticleTemplate`))
    (`SceneComponent.SetWorldScale3D` (`local.CurrentParticleEffect`) (`KismetMathLibrary.Conv_DoubleToVector` (`self.Shield_Scale`)))
    (`SceneComponent.K2_AddLocalOffset` (`local.CurrentParticleEffect`) (`KismetMathLibrary.MakeVector` (`self.Shield_Radius`)) false false)
    (`SceneComponent.K2_AttachToComponent` (`local.CurrentParticleEffect`) (`self.Arrow`) "None" "KeepRelative" "KeepRelative" "KeepRelative" true)))